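; BP_HealthComponent is a component that tracks the current and maximum health of its owner.
; It resets health to the maximum on BeginPlay.
; GetDamage subtracts the absolute damage amount and clamps the result between zero and the maximum.
; It then broadcasts OnHealtZero when health reaches zero, or OnGetDamage otherwise, so other Blueprints can react.
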(event `self.ReceiveBeginPlay`
  (`self.ResetHealth`))

(fn `GetDamage`
  (params (DamageAmount :type "Float (double-precision)"))
  (bind _output_get (set `self.CurrentHealth` (`KismetMathLibrary.FClamp` (- (`self.CurrentHealth`) (`KismetMathLibrary.Abs` DamageAmount)) 0.0 (`self.MaxHealth`))))
  (if (== _output_get 0.0)
    (`self.OnHealtZero`)
    (else
      (`self.OnGetDamage`))))

(fn `ResetHealth`
  (set `self.CurrentHealth` (`self.MaxHealth`)))