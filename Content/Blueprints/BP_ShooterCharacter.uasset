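; BP_ShooterCharacter is a shooter character Blueprint that exposes its mesh and the endpoints of a firing line.
; RetrieveCharacterMesh returns the Mesh component, while GetFireStart returns the capsule's world location.
; GetFireEnd projects a given Range from that location along the capsule's forward vector, so aim follows the capsule's facing rather than a camera or muzzle.
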(fn `GetFireEnd`
  (params (Range :type "Float (double-precision)"))
  (returns (End :type "Vector Structure"))
  (bind _capsulecomponent (`self.CapsuleComponent`))
  (return (+ (`SceneComponent.K2_GetComponentLocation` _capsulecomponent) (* Range (`SceneComponent.GetForwardVector` _capsulecomponent)))))

(fn `GetFireStart`
  (returns (StartPos :type "Vector Structure"))
  (return (`SceneComponent.K2_GetComponentLocation` (`self.CapsuleComponent`))))

(fn `RetrieveCharacterMesh`
  (returns (Mesh :type "SkeletalMeshComponent Object Reference"))
  (return (`self.Mesh`)))

(fn `UserConstructionScript`)