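; BP_TrashController is a trigger volume that freezes a set of trash actors while the first-person character is inside its box.
; Box overlap begin clears MovementAllowed on every valid actor in TrashList, and overlap end sets it back to true.
; The exit path also prints a debug string after re-enabling movement.
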(event `self.Box.OnComponentBeginOverlap`
  (params (OverlappedComponent :type "PrimitiveComponent Object Reference") (OtherActor :type "Actor Object Reference") (OtherComp :type "PrimitiveComponent Object Reference") (OtherBodyIndex :type Integer) (bFromSweep :type Boolean) (SweepResult :type "HitResult Structure (by ref)"))
  (cast `/Game/Blueprints/FirstPerson/BP_FirstPersonCharacter` OtherActor)
  (for _array_element (`self.TrashList`)
    (`/Engine/EditorBlueprintResources/StandardMacros.IsValid` _array_element
      (:`Is Valid`
        (set `/Game/Veronica/Trash.MovementAllowed` false _array_element)))))

(event `self.Box.OnComponentEndOverlap`
  (params (OverlappedComponent :type "PrimitiveComponent Object Reference") (OtherActor :type "Actor Object Reference") (OtherComp :type "PrimitiveComponent Object Reference") (OtherBodyIndex :type Integer))
  (cast `/Game/Blueprints/FirstPerson/BP_FirstPersonCharacter` OtherActor)
  (for _array_element (`self.TrashList`)
    (`/Engine/EditorBlueprintResources/StandardMacros.IsValid` _array_element
      (:`Is Valid`
        (set `/Game/Veronica/Trash.MovementAllowed` true _array_element))))
  (`KismetSystemLibrary.PrintString` "set all to true"))

(fn `UserConstructionScript`)