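; BP_Mine is a mine actor that deals area damage to shooter characters and then destroys itself.
; On the OnHit event it runs a sphere overlap at its location for BP_ShooterCharacter pawns within DamageRadius and draws a debug sphere of that radius.
; Each valid actor found with a BP_HealthComponent receives DamageAmount through GetDamage.
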(event `/Game/Blueprints/Gameplay/BPI_HitBehaviour.OnHit`
  (bind _returnvalue (`self.K2_GetActorLocation`))
  (bind _outactors (`KismetSystemLibrary.SphereOverlapActors` _returnvalue (`self.DamageRadius`) (`|MakeArray` "ObjectTypeQuery3" :!type "EObjectTypeQuery Enum") "/Game/Blueprints/BP_ShooterCharacter.BP_ShooterCharacter_C"))
  (`KismetSystemLibrary.DrawDebugSphere` _returnvalue (`self.DamageRadius`) 12 (struct :`R` 1.0 :`G` 0.26489 :`B` 0.370328 :`A` 1.0) 5.0)
  (for _array_element _outactors
    (`/Engine/EditorBlueprintResources/StandardMacros.IsValid` _array_element
      (:`Is Valid`
        (bind _returnvalue_2 (`self.GetComponentByClass` _array_element "/Game/Blueprints/Components/BP_HealthComponent.BP_HealthComponent_C"))
        (`/Engine/EditorBlueprintResources/StandardMacros.IsValid` _returnvalue_2
          (:`Is Valid`
            (`/Game/Blueprints/Components/BP_HealthComponent.GetDamage` _returnvalue_2 (`self.DamageAmount`)))))))
  (`self.K2_DestroyActor`))

(fn `UserConstructionScript`)