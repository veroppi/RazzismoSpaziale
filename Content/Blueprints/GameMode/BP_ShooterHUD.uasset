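; BP_ShooterHUD is the shooter HUD that shows a crosshair only while the player character has a rifle.
; On BeginPlay it creates the BP_Crosshair widget, adds it to the viewport and caches the player's BP_ShooterCharacter.
; It binds to the character's OnChangeWeapon dispatcher and runs the handler once at start, so crosshair visibility follows HasRifle without polling on Tick.
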(event `self.ReceiveBeginPlay`
  (bind _returnvalue (`|CreateWidget` "/Game/Blueprints/GameMode/BP_Crosshair.BP_Crosshair_C"))
  (bind _output_get (set `self.CrosshairWidget` _returnvalue))
  (`UserWidget.AddToViewport` _output_get 0)
  (bind _asbp_shooter_character (cast `/Game/Blueprints/BP_ShooterCharacter` (`GameplayStatics.GetPlayerPawn` 0)))
  (bind _output_get_2 (set `self.CharacterRef` _asbp_shooter_character))
  (add `/Game/Blueprints/BP_ShooterCharacter.OnChangeWeapon` _output_get_2 (delegate `OnChangeWeapon`))
  (`self.OnChangeWeapon`))

(event `OnChangeWeapon`
  (`self.SetCrosshairVisibility` (`/Game/Blueprints/BP_ShooterCharacter.bHasRifle` (`self.CharacterRef`))))

(fn `SetCrosshairVisibility`
  (params (NewVisibility :type Boolean))
  (bind _crosshairwidget (`self.CrosshairWidget`))
  (`/Engine/EditorBlueprintResources/StandardMacros.IsValid` _crosshairwidget
    (:`Is Valid`
      (if NewVisibility
        (`Widget.SetVisibility` _crosshairwidget "Visible")
        (else
          (`Widget.SetVisibility` _crosshairwidget "Hidden"))))))

(fn `UserConstructionScript`)