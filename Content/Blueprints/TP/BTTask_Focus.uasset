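; Behavior tree task that turns the AI-controlled pawn to face the first player's pawn.
; On execute it stores the current rotation and a look-at rotation, so the target is not tracked as the player moves.
; Tick linearly eases between them, using RotationSpeed as a duration, then finishes successfully.
; It fails if either pawn is invalid at start.
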(event `self.ReceiveExecuteAI`
  (params (OwnerController :type "AIController Object Reference") (ControlledPawn :type "Pawn Object Reference"))
  (bind _returnvalue (`GameplayStatics.GetPlayerPawn` 0))
  (set `self.elapsedTime` 0.0)
  (`/Engine/EditorBlueprintResources/StandardMacros.IsValid` ControlledPawn
    (:`Is Valid`
      (set `self.StartRotation` (`Actor.K2_GetActorRotation` ControlledPawn))
      (`/Engine/EditorBlueprintResources/StandardMacros.IsValid` _returnvalue
        (:`Is Valid`
          (set `self.EndRotation` (`KismetMathLibrary.FindLookAtRotation` (`Actor.K2_GetActorLocation` ControlledPawn) (`Actor.K2_GetActorLocation` _returnvalue))))
        (:`Is Not Valid`
          (`self.FinishExecute` false))))
    (:`Is Not Valid`
      (`self.FinishExecute` false))))

(event `self.ReceiveTickAI`
  (params (OwnerController :type "AIController Object Reference") (ControlledPawn :type "Pawn Object Reference") (DeltaSeconds :type "Float (single-precision)"))
  (bind _output_get (set `self.elapsedTime` (+ DeltaSeconds (`self.elapsedTime`))))
  (`Actor.K2_SetActorRotation` ControlledPawn (`|EaseFunction` "Linear" (/ _output_get (`self.RotationSpeed`)) (`self.StartRotation`) (`self.EndRotation`)) false)
  (if (>= _output_get (`self.RotationSpeed`))
    (`self.FinishExecute` true)))