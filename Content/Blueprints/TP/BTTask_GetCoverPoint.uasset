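; Behavior tree task that picks the spot on the far side of the target cover from the player for an enemy to move to.
; It asks the BP_Cover in BBTargetCover for its point closest to the player, then mirrors it in XY around the cover's origin.
; The result goes into BBDestination, with debug spheres at both points.
; Non-enemy pawns fail; a failed cover cast never finishes the task.
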(event `self.ReceiveExecuteAI`
  (params (OwnerController :type "AIController Object Reference") (ControlledPawn :type "Pawn Object Reference"))
  (bind _returnvalue (`BTFunctionLibrary.GetBlackboardValueAsActor` (`self.BB_TargetCover`)))
  (bind _returnvalue_2 (`Actor.K2_GetActorLocation` _returnvalue))
  (cast `/Game/Blueprints/TP/BP_enemyBase` ControlledPawn
    (:`then`
      (bind _asbp_cover (cast `/Game/Blueprints/Gameplay/BP_Cover` _returnvalue))
      (bind _outpointonbody (`/Game/Blueprints/Gameplay/BP_Cover.GetClosestFromPoint` _asbp_cover (`Actor.K2_GetActorLocation` (`GameplayStatics.GetPlayerPawn` 0))))
      (`KismetSystemLibrary.DrawDebugSphere` _outpointonbody 20.0 12 (struct :`R` 0.495823 :`G` 0.36041 :`B` 1.0 :`A` 1.0) 0.1)
      (bind (_returnvalue_x _returnvalue_y _returnvalue_z) (`KismetMathLibrary.BreakVector` (- _outpointonbody _returnvalue_2)))
      (bind _returnvalue_3 (+ (`KismetMathLibrary.MakeVector` (* _returnvalue_x -1.0) (* _returnvalue_y -1.0) _returnvalue_z) _returnvalue_2))
      (`KismetSystemLibrary.DrawDebugSphere` _returnvalue_3 20.0 12 (struct :`R` 1.0 :`G` 0.345723 :`B` 0.29985 :`A` 1.0) 0.1)
      (`BTFunctionLibrary.SetBlackboardValueAsVector` (`self.BB_Destination`) _returnvalue_3)
      (`self.FinishExecute` true))
    (:`CastFailed`
      (`self.FinishExecute` false))))