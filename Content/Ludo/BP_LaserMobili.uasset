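; Moving laser actor that shuttles between its start location and an offset marker position, pausing at each end.
; Tick drives Move, which lerps location over Duration and flips direction on arrival, then a timer re-enables movement after WaitTime.
; Each moving tick looks up BP_ShooterCharacter: when its SpeedySpeed flag is set, the laser moves slower and waits longer, otherwise it runs faster with shorter pauses.
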(event `self.ReceiveBeginPlay`
  (bind _returnvalue (`self.K2_GetActorLocation`))
  (set `self.StartPosition` _returnvalue)
  (set `self.EndPosition` (+ _returnvalue (`self.EndPostionMarker`)))
  (set `self.bGoUp` true)
  (set `self.bCanMove` false)
  (`KismetSystemLibrary.K2_SetTimerDelegate` (delegate `OnWaitTime`) (`self.WaitTime`)))

(event `OnWaitTime`
  (set `self.bCanMove` true))

(event `self.ReceiveTick`
  (params (DeltaSeconds :type "Float (single-precision)"))
  (if (`self.bCanMove`)
    (bind _returnvalue (`GameplayStatics.GetActorOfClass` "/Game/Blueprints/BP_ShooterCharacter.BP_ShooterCharacter_C"))
    (castclass `/Game/Blueprints/BP_ShooterCharacter` (`GameplayStatics.GetObjectClass` _returnvalue))
    (if (`/Game/Blueprints/BP_ShooterCharacter.SpeedySpeed` _returnvalue)
      (set `self.WaitTime` 0.7)
      (bind _hasarrived (`self.Move` (* DeltaSeconds 3.0)))
      (if _hasarrived
        (set `self.bCanMove` false :!label _label)
        (`KismetSystemLibrary.K2_SetTimerDelegate` (delegate `OnWaitTime`) (`self.WaitTime`)))
      (else
        (set `self.WaitTime` 0.3)
        (bind _hasarrived_2 (`self.Move` (* DeltaSeconds 12.0)))
        (if _hasarrived_2
          (goto _label))))))

(fn `Move`
  (params (DeltaSeconds :type "Float (double-precision)"))
  (returns (HasArrived :type Boolean))
  (bind _returnvalue (/ (`self.elapsedTime`) (`self.Duration`)))
  (bind _output_get (set `self.elapsedTime` (+ DeltaSeconds (`self.elapsedTime`))))
  (if (>= _output_get (`self.Duration`))
    (set `self.elapsedTime` 0.0)
    (set `self.bGoUp` (not (`self.bGoUp`)))
    (return true)
    (else
      (if (`self.bGoUp`)
        (`self.K2_SetActorLocation` (`KismetMathLibrary.VLerp` (`self.StartPosition`) (`self.EndPosition`) _returnvalue))
        (else
          (`self.K2_SetActorLocation` (`KismetMathLibrary.VLerp` (`self.EndPosition`) (`self.StartPosition`) _returnvalue))))
      (return false))))

(fn `PrintActorName`
  (params (StringToPrint :type String) (TargetObject :type "Object Object Reference"))
  (`KismetSystemLibrary.PrintString` (`KismetStringLibrary.Concat_StrStr` StringToPrint (`KismetSystemLibrary.GetDisplayName` TargetObject))))

(fn `Return_Sum`
  (params (N1 :type "Float (double-precision)" :default 5.0) (N2 :type "Float (double-precision)" :default 10.0))
  (returns (Somma :type "Float (double-precision)"))
  (return (+ N1 N2)))

(fn `UserConstructionScript`)