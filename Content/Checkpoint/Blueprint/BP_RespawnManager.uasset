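; Respawn manager that restores player state from RespawnData after a short timer delay on BeginPlay.
; On a first spawn it only copies the saved WeaponsCount to the BP_ShooterCharacter's weapon, if that weapon is valid.
; Otherwise it moves BP_FirstPersonCharacter to the saved position and rotation, then restores its weapon count.
; Ending play in editor sets the FirstSpawn flag back to true.
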(event `StartingSpawnEvent`
  (bind _returnvalue (`GameplayStatics.GetActorOfClass` "/Game/Blueprints/BP_ShooterCharacter.BP_ShooterCharacter_C"))
  (bind _weapon (`/Game/Blueprints/BP_ShooterCharacter.Weapon` _returnvalue))
  (`/Game/EditorBlueprintResources/StandardMacros.IsValid` _weapon
    (:`Is Valid`
      (set `/Game/Blueprints/Components/BP_Weapon_Component.WeaponsCount` (`/Game/Checkpoint/Blueprint/PDA_Checkpoint.WeaponsCount` (`self.RespawnData`)) _weapon))))

(event `self.ReceiveEndPlay`
  (params (EndPlayReason :type "EEndPlayReason Enum" :default "Destroyed"))
  (if (`|EnumEquality` EndPlayReason "EndPlayInEditor")
    (`self.ResetRespawnData`)))

(event `self.ReceiveBeginPlay`
  (if (`/Game/Checkpoint/Blueprint/PDA_Checkpoint.FirstSpawn` (`self.RespawnData`))
    (`KismetSystemLibrary.K2_SetTimerDelegate` (delegate `StartingSpawnEvent`) (`self.RespawnDelay`))
    (else
      (`KismetSystemLibrary.K2_SetTimerDelegate` (delegate `Respawn Event`) (`self.RespawnDelay`)))))

(event `Respawn Event`
  (bind _respawndata (`self.RespawnData`))
  (bind _returnvalue (`GameplayStatics.GetActorOfClass` "/Game/Blueprints/FirstPerson/BP_FirstPersonCharacter.BP_FirstPersonCharacter_C"))
  (`self.K2_SetActorLocation` _returnvalue (`/Game/Checkpoint/Blueprint/PDA_Checkpoint.SpawnPosition` _respawndata) false false)
  (`self.K2_SetActorRotation` _returnvalue (`/Game/Checkpoint/Blueprint/PDA_Checkpoint.SpawnRotation` _respawndata) false)
  (set `/Game/Blueprints/Components/BP_Weapon_Component.WeaponsCount` (`/Game/Checkpoint/Blueprint/PDA_Checkpoint.WeaponsCount` _respawndata) (`/Game/Blueprints/BP_ShooterCharacter.Weapon` _returnvalue)))

(fn `ResetRespawnData`
  (set `/Game/Checkpoint/Blueprint/PDA_Checkpoint.FirstSpawn` true (`self.RespawnData`)))

(fn `UserConstructionScript`)