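; BP_LaserMobili_Orizzontali1 is a moving laser hazard that shuttles between its start location and an offset marker, damaging the player on overlap.
; Tick calls Move, which lerps the position over Duration and flips direction at each end, then a timer pauses it for WaitTime.
; The shooter character's SpeedySpeed flag selects slower movement and longer pauses.
; Overlap deals heavy damage through PlayerHealthComponent on BP_FirstPersonCharacter, then grants brief laser immunity.
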(event `self.ReceiveBeginPlay`
  (bind _returnvalue (`self.K2_GetActorLocation`))
  (set `self.StartPosition` _returnvalue)
  (set `self.EndPosition` (+ _returnvalue (`self.EndPostionMarker`)))
  (set `self.bGoUp` true)
  (set `self.bCanMove` false)
  (`KismetSystemLibrary.K2_SetTimerDelegate` (delegate `OnWaitTime`) (`self.WaitTime`)))

(event `OnWaitTime`
  (set `self.bCanMove` true))

(event `self.ReceiveTick`
  (params (DeltaSeconds :type "Float (single-precision)"))
  (if (`self.bCanMove`)
    (bind _returnvalue (`GameplayStatics.GetActorOfClass` "/Game/Blueprints/BP_ShooterCharacter.BP_ShooterCharacter_C"))
    (castclass `/Game/Blueprints/BP_ShooterCharacter` (`GameplayStatics.GetObjectClass` _returnvalue))
    (if (`/Game/Blueprints/BP_ShooterCharacter.SpeedySpeed` _returnvalue)
      (set `self.WaitTime` 0.7)
      (bind _hasarrived (`self.Move` (* DeltaSeconds 9.0)))
      (if _hasarrived
        (set `self.bCanMove` false :!label _label)
        (`KismetSystemLibrary.K2_SetTimerDelegate` (delegate `OnWaitTime`) (`self.WaitTime`)))
      (else
        (set `self.WaitTime` 0.3)
        (bind _hasarrived_2 (`self.Move` (* DeltaSeconds 36.0)))
        (if _hasarrived_2
          (goto _label))))))

(event `self.ReceiveActorBeginOverlap`
  (params (OtherActor :type "Actor Object Reference"))
  (if (`self.ActorHasTag` OtherActor "Player")
    (bind _returnvalue (`GameplayStatics.GetActorOfClass` "/Game/Blueprints/FirstPerson/BP_FirstPersonCharacter.BP_FirstPersonCharacter_C"))
    (bind _playerhealthcomponent (`/Game/Blueprints/FirstPerson/BP_FirstPersonCharacter.PlayerHealthComponent` _returnvalue))
    (if (not (`/Game/Ludo/PlayerHealthComponent.LaserImmune` _playerhealthcomponent))
      (`/Game/Ludo/PlayerHealthComponent.AddHealth` _playerhealthcomponent -120.0)
      (set `/Game/Ludo/PlayerHealthComponent.LaserImmune` true _playerhealthcomponent)
      (`KismetSystemLibrary.Delay` 0.5)
      (`/Engine/EditorBlueprintResources/StandardMacros.IsValid` _returnvalue
        (:`Is Valid`
          (set `/Game/Ludo/PlayerHealthComponent.LaserImmune` false _playerhealthcomponent))))))

(fn `Move`
  (params (DeltaSeconds :type "Float (double-precision)"))
  (returns (HasArrived :type Boolean))
  (bind _returnvalue (/ (`self.elapsedTime`) (`self.Duration`)))
  (bind _output_get (set `self.elapsedTime` (+ DeltaSeconds (`self.elapsedTime`))))
  (if (>= _output_get (`self.Duration`))
    (set `self.elapsedTime` 0.0)
    (set `self.bGoUp` (not (`self.bGoUp`)))
    (return true)
    (else
      (if (`self.bGoUp`)
        (`self.K2_SetActorLocation` (`KismetMathLibrary.VLerp` (`self.StartPosition`) (`self.EndPosition`) _returnvalue))
        (else
          (`self.K2_SetActorLocation` (`KismetMathLibrary.VLerp` (`self.EndPosition`) (`self.StartPosition`) _returnvalue))))
      (return false))))

(fn `PrintActorName`
  (params (StringToPrint :type String) (TargetObject :type "Object Object Reference"))
  (`KismetSystemLibrary.PrintString` (`KismetStringLibrary.Concat_StrStr` StringToPrint (`KismetSystemLibrary.GetDisplayName` TargetObject))))

(fn `Return_Sum`
  (params (N1 :type "Float (double-precision)" :default 5.0) (N2 :type "Float (double-precision)" :default 10.0))
  (returns (Somma :type "Float (double-precision)"))
  (return (+ N1 N2)))

(fn `UserConstructionScript`)